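; TronTrail lays down a Tron-style trail of spline meshes behind a moving Trail component.
; BeginPlay clears the spline, seeds it at Trail's world position and starts a looping AddWaypoint timer.
; While ShouldGrow is set, each tick of that timer appends a world-space point once Trail moves far enough from the last one.
; Each new point spawns a spline mesh spanning the last two points, using their tangents.
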(event Custom|AddWaypoint
  (bind _spline (Variables|Default|GetSpline))
  (bind _trail (Variables|Default|GetTrail))
  (bind _spline_2 (Variables|Default|GetSpline))
  (bind _returnvalue (Spline|GetNumberOfSplinePoints _spline_2))
  (bind _returnvalue_2 (- _returnvalue 2))
  (bind (_location _tangent) (Spline|GetLocationandTangentatSplinePoint _spline_2 _returnvalue_2 "World"))
  (bind _returnvalue_3 (+ _returnvalue_2 1))
  (bind (_location_2 _tangent_2) (Spline|GetLocationandTangentatSplinePoint _spline_2 _returnvalue_3 "World"))
  (if (Utilities|IsValid _trail)
    (if (and (Variables|Default|GetShouldGrow) (> (Math|Vector|Distance(Vector) (Transformation|GetWorldLocation _trail) (Spline|GetLocationatSplinePoint _spline (Spline|GetNumberOfSplinePoints _spline) "World")) 25.0))
      (Spline|AddSplinePoint (Variables|Default|GetSpline) (Transformation|GetWorldLocation (Variables|Default|GetTrail)) "World" true)
      (bind _returnvalue_4 (AddComponent|AddSplineMeshComponent true))
      (SplineMesh|SetStartandEnd _returnvalue_4 _location _tangent _location_2 _tangent_2 true :!class /Script/Engine.SplineMeshComponent))))

(event EventBeginPlay
  (bind _spline (Variables|Default|GetSpline))
  (bind _returnvalue (Spline|GetNumberOfSplinePoints _spline))
  (bind _returnvalue_2 (- _returnvalue 2))
  (bind (_location _tangent) (Spline|GetLocationandTangentatSplinePoint _spline _returnvalue_2 "World"))
  (bind _returnvalue_3 (+ _returnvalue_2 1))
  (bind (_location_2 _tangent_2) (Spline|GetLocationandTangentatSplinePoint _spline _returnvalue_3 "World"))
  (bind _returnvalue_4 (Utilities|Time|SetTimerbyEvent (delegate Custom|AddWaypoint) 0.075 true))
  (Variables|Default|SetTimer%20Handle _returnvalue_4)
  (Spline|ClearSplinePoints (Variables|Default|GetSpline) true)
  (if (Utilities|IsValid (Variables|Default|GetTrail))
    (Spline|AddSplinePoint (Variables|Default|GetSpline) (Transformation|GetWorldLocation (Variables|Default|GetTrail)) "World" true)
    (bind _returnvalue_5 (AddComponent|AddSplineMeshComponent true))
    (SplineMesh|SetStartandEnd _returnvalue_5 _location _tangent _location_2 _tangent_2 true :!class /Script/Engine.SplineMeshComponent)))

(fn ConstructionScript)