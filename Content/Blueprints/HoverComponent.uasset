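; A hover thruster scene component that pushes a physics-driven parent component away from the surface beneath it.
; Initialize stores the parent along with hover height, force and damping settings.
; Each tick it traces down its local up axis and applies force at its own location along the hit normal, fading linearly to zero at hover height.
; A hit also sets the parent's damping, which is not reset on a miss.
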(event Custom|Initialize
  (params (Parent :type Primitive%20Component%20Object%20Reference) (HoverHeight :type Float%20%28single-precision%29) (HoverForce :type Float%20%28single-precision%29) (LinearDamping :type Float%20%28single-precision%29) (AngularDamping :type Float%20%28single-precision%29))
  (Variables|Default|SetParent Parent)
  (Variables|Default|SetHover%20Height HoverHeight)
  (Variables|Default|SetHoverForce HoverForce)
  (Variables|Default|SetLinearDamping LinearDamping)
  (Variables|Default|SetAngularDamping AngularDamping))

(event EventTick
  (params (DeltaSeconds :type Float%20%28single-precision%29))
  (bind _returnvalue (Transformation|GetWorldLocation))
  (bind (_outhit _returnvalue_2) (Collision|LineTraceByChannel _returnvalue (+ _returnvalue (* (Math|Vector|GetUpVector) (* (Variables|Default|GetHover%20Height) -1.0))) "TraceTypeQuery1" false (Utilities|Array|MakeArray (Components|GetOwner (Variables|Default|GetParent))) "ForOneFrame"))
  (if _returnvalue_2
    (Class|PrimitiveComponent|AddForceatLocation (Variables|Default|GetParent) (* (.ImpactNormal (Collision|BreakHitResult _outhit)) (Math|Float|Lerp (Variables|Default|GetHoverForce) 0.0 (/ (.Distance (Collision|BreakHitResult _outhit)) (Variables|Default|GetHover%20Height)))) (Transformation|GetWorldLocation) "None")
    (Class|PrimitiveComponent|SetLinearDamping (Variables|Default|GetParent) (Variables|Default|GetLinearDamping))
    (Class|PrimitiveComponent|SetAngularDamping (Variables|Default|GetParent) (Variables|Default|GetAngularDamping))))