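; Player-driven hover vehicle that floats on four corner hover components, set up at BeginPlay with stronger lift at the rear.
; Forward input drives a thruster along the body's forward axis, while strafe pushes sideways at two corner points.
; Turning applies opposed forces at diagonal corners, with a sign intended to flip when reversing.
; Both mouse axes feed one spring-arm pitch and yaw rotation, and Tick prints forward speed for debugging.
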(event EventBeginPlay
  (Default|Initialize (Variables|Default|GetHoverComponent_RR) (Variables|Default|GetBody) (Variables|Default|GetHoverHeight) 9e+05 5.0 8.0)
  (Default|Initialize (Variables|Default|GetHoverComponent_FL) (Variables|Default|GetBody) (Variables|Default|GetHoverHeight) 7e+05 5.0 8.0))

(event EventTick
  (params (DeltaSeconds :type Float%20%28single-precision%29))
  (Development|PrintString (Utilities|String|ToString(Float) (Math|Vector|DotProduct (Transformation|GetVelocity) (Math|Vector|GetForwardVector (Variables|Default|GetBody))))))

(event Input|AxisEvents|InputAxisStrafe
  (params (AxisValue :type Float%20%28single-precision%29))
  (bind _body (Variables|Default|GetBody))
  (bind _rr (Variables|Default|GetRR))
  (bind _strafethrust (Variables|Default|GetStrafeThrust))
  (bind _fl (Variables|Default|GetFL))
  (bind _fr (Variables|Default|GetFR))
  (bind _rl (Variables|Default|GetRL))
  (bind _returnvalue (Math|Vector|GetRightVector _body))
  (bind _returnvalue_2 (* AxisValue _strafethrust))
  (bind _returnvalue_3 (* _returnvalue_2 _returnvalue))
  (if (> AxisValue 0.0)
    (Class|PrimitiveComponent|AddForceatLocation _fr _returnvalue_3 (Transformation|GetWorldLocation _fr) "None")
    (Class|PrimitiveComponent|AddForceatLocation _rr _returnvalue_3 (Transformation|GetWorldLocation _rr) "None")
    (else
      (Class|PrimitiveComponent|AddForceatLocation _rl _returnvalue_3 (Transformation|GetWorldLocation _rl) "None")
      (Class|PrimitiveComponent|AddForceatLocation _fl _returnvalue_3 (Transformation|GetWorldLocation _fl) "None"))))

(event Input|AxisEvents|InputAxisForward
  (params (AxisValue :type Float%20%28single-precision%29))
  (Physics|AddForce (Variables|Default|GetThruster) (* (Math|Vector|GetForwardVector (Variables|Default|GetBody)) (* AxisValue (Variables|Default|GetForwardThrust))) "None" true))

(event Input|AxisEvents|InputAxisRight
  (params (AxisValue :type Float%20%28single-precision%29))
  (bind _rr (Variables|Default|GetRR))
  (bind _fl (Variables|Default|GetFL))
  (bind _body (Variables|Default|GetBody))
  (bind _fr (Variables|Default|GetFR))
  (bind _rl (Variables|Default|GetRL))
  (bind _returnvalue (Physics|GetPhysicsLinearVelocity _body "None"))
  (if (or (Math|Float|NearlyEqual(Float) (Math|Vector|DotProduct _returnvalue (Math|Vector|GetForwardVector _body)) 0.0 -1e+01) (Math|Float|NearlyEqual(Float) (Math|Vector|DotProduct _returnvalue (Math|Vector|GetForwardVector _body)) 0.0 1e+01))
    (Variables|Default|SetCorrect%20Rotation 1.0)
    (elif (> (Math|Vector|DotProduct _returnvalue (Math|Vector|GetForwardVector _body)) 0.0)
      (Variables|Default|SetCorrect%20Rotation 1.0)
      (else
        (Variables|Default|SetCorrect%20Rotation -1.0))))
  (if (> AxisValue 0.0)
    (Class|PrimitiveComponent|AddForceatLocation _fl (* (* (* AxisValue (Variables|Default|GetCorrect%20Rotation)) (Variables|Default|GetRotationThrust)) (Math|Vector|GetRightVector (Variables|Default|GetBody))) (Transformation|GetWorldLocation _fl) "None")
    (Class|PrimitiveComponent|AddForceatLocation _rr (* (* (* (* AxisValue (Variables|Default|GetCorrect%20Rotation)) (Variables|Default|GetRotationThrust)) (Math|Vector|GetRightVector (Variables|Default|GetBody))) -1.0) (Transformation|GetWorldLocation _rr) "None")
    (else
      (Class|PrimitiveComponent|AddForceatLocation _fr (* (* (* AxisValue (Variables|Default|GetCorrect%20Rotation)) (Variables|Default|GetRotationThrust)) (Math|Vector|GetRightVector (Variables|Default|GetBody))) (Transformation|GetWorldLocation _fr) "None")
      (Class|PrimitiveComponent|AddForceatLocation _rl (* (* (* (* AxisValue (Variables|Default|GetCorrect%20Rotation)) (Variables|Default|GetRotationThrust)) (Math|Vector|GetRightVector (Variables|Default|GetBody))) -1.0) (Transformation|GetWorldLocation _rl) "None"))))

(event Input|MouseEvents|MouseX
  (params (AxisValue :type Float%20%28single-precision%29))
  (Transformation|AddRelativeRotation (Variables|Default|GetSpringArm) (Math|Rotator|MakeRotator 0.0 (* (stale Input|MouseEvents|MouseY AxisValue) -1.0) AxisValue) false false))

(event Input|MouseEvents|MouseY
  (params (AxisValue :type Float%20%28single-precision%29))
  (Transformation|AddRelativeRotation (Variables|Default|GetSpringArm) (Math|Rotator|MakeRotator 0.0 (* AxisValue -1.0) (stale Input|MouseEvents|MouseX AxisValue)) false false))

(fn ConstructionScript)